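; BP_LMAGameMode is the game mode Blueprint that runs the match countdown and shows the end-of-time menu.
; On BeginPlay it starts a looping one-second timer whose event decrements GameTime.
; When GameTime reaches zero, it clears GameTimerHandle and adds a WBP_TimerEndMenu widget to the viewport.
; The graph does not show the timer's handle being stored in GameTimerHandle.
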(event Custom|CustomEvent
  (bind _output_get (Variables|Default|SetGameTime (- (Variables|Default|GetGameTime) 1)))
  (if (== _output_get 0)
    (Utilities|Time|ClearandInvalidateTimerbyHandle (Variables|Default|GetGameTimerHandle))
    (bind _returnvalue (UserInterface|CreateWidget "/Game/LeaveMeAlone/Core/Widgets/UI/WBP_TimerEndMenu.WBP_TimerEndMenu_C"))
    (UserInterface|Viewport|AddtoViewport _returnvalue 0)))

(event EventTick
  (params (DeltaSeconds :type Float%20%28single-precision%29)))

(event EventBeginPlay
  (Utilities|Time|SetTimerbyEvent (delegate Custom|CustomEvent) 1.0 true))

(fn ConstructionScript)